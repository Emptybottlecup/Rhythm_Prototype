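; Rhythm-game enemy that runs forward in a line and gets decapitated when the player attacks it.
; Move sets walk speed from SplineDistance and sends it straight ahead with AI MoveTo.
; Tick triggers Death when EnemyRadius is Big Radius and the player attacks on the same line, consuming the attack.
; Death ragdolls the body, spawns gore Niagara effects and releases a velocity-clamped physics head before delayed destruction.
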(event `self.ReceiveBeginPlay`)

(event `Move`
  (set `CharacterMovementComponent.MaxWalkSpeed` (/ (`self.Spline Distance`) 5.0) (`self.CharacterMovement`))
  (`|AIMoveTo` self (+ (`self.K2_GetActorLocation`) (* (`self.GetActorForwardVector`) 3000.0)) null))

(event `Death`
  (bind _head (`self.Head`))
  (bind _mesh (`self.Mesh`))
  (`SkeletalMeshComponent.SetSkeletalMeshAsset` _mesh "/Game/AAAModularSoldier/Modules/ModularSoldierVol_1/Cutting/body.body")
  (`PrimitiveComponent.SetSimulatePhysics` _mesh true)
  (`NiagaraFunctionLibrary.SpawnSystemAttached` "/Game/BloodPack/BrainBurst/Niagara/NS_BrainBurst.NS_BrainBurst" _mesh "neck_01" (0.0 0.0 0.0) (struct) "KeepRelativeOffset")
  (`NiagaraFunctionLibrary.SpawnSystemAttached` "/Game/BloodPack/Amputated/Niagara/NS_AmputatedHead.NS_AmputatedHead" _mesh "neck_01" (0.0 0.0 0.0) (struct) "KeepRelativeOffset")
  (`SceneComponent.SetVisibility` _head true false)
  (`PrimitiveComponent.SetSimulatePhysics` _head true)
  (`PrimitiveComponent.SetCollisionEnabled` _head "PhysicsOnly")
  (`PrimitiveComponent.SetCollisionEnabled` (`self.CapsuleComponent`) "NoCollision")
  (set `self.DeathState` true)
  (`KismetSystemLibrary.Delay` 1.5)
  (`self.K2_DestroyActor`))

(event `self.ReceiveTick`
  (params (DeltaSeconds :type "Float (single-precision)"))
  (bind _head (`self.Head`))
  (`|ExecutionSequence`
    (:`then_0`
      (switch `/Game/RhythmGame/Enum/E_EnemyRadiusDamage` (`self.EnemyRadius`)
        (:`NewEnumerator1`
          (bind _returnvalue (`GameplayStatics.GetActorOfClass` "/Game/RhythmGame/Blueprints/BP_ThirdPersonCharacter.BP_ThirdPersonCharacter_C"))
          (if (and (== (`KismetMathLibrary.Conv_ByteToInt` (`/Game/RhythmGame/Blueprints/BP_ThirdPersonCharacter.PlayerStateLine` _returnvalue)) (`KismetMathLibrary.Conv_ByteToInt` (`self.EnemyLine`))) (`/Game/RhythmGame/Blueprints/BP_ThirdPersonCharacter.Attacking` _returnvalue))
            (`self.Death`)
            (set `/Game/RhythmGame/Blueprints/BP_ThirdPersonCharacter.Attacking` false _returnvalue)))))
    (:`then_1`
      (if (`self.DeathState`)
        (bind _returnvalue_2 (`PrimitiveComponent.GetPhysicsLinearVelocity` _head "None"))
        (`PrimitiveComponent.SetPhysicsLinearVelocity` _head (`KismetMathLibrary.MakeVector` (`KismetMathLibrary.FClamp` (.x _returnvalue_2) -50.0 50.0) (`KismetMathLibrary.FClamp` (.y _returnvalue_2) -50.0 50.0) (`KismetMathLibrary.FClamp` (.z _returnvalue_2) -500.0 130.0)) false "None")))))

(fn `UserConstructionScript`)