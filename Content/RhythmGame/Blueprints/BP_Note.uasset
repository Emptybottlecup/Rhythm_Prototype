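; BP_Note is a rhythm game note actor that travels along one of three splines from the level's BP_Spline, picked at random on BeginPlay.
; MoveNote drives a timeline, scaled by TimeToComplete, that sets position and rotation along the spline.
; The first update spawns a BP_Enemy at the note, passes it the spline length and calls Move.
; The note destroys itself when the timeline finishes or BP_ThirdPersonCharacter overlaps its sphere.
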(event `self.ReceiveBeginPlay`
  (bind _spline (`self.Spline`))
  (bind _returnvalue (`GameplayStatics.GetActorOfClass` "/Game/RhythmGame/Blueprints/BP_Spline.BP_Spline_C"))
  (set `self.Spline` _returnvalue)
  (set `self.SplineComp` (select `int` (`KismetMathLibrary.RandomIntegerInRange` 0 2) :`0` (`/Game/RhythmGame/Blueprints/BP_Spline.Spline2` _spline) :`1` (`/Game/RhythmGame/Blueprints/BP_Spline.Spline1` _spline) :`2` (`/Game/RhythmGame/Blueprints/BP_Spline.Spline` _spline))))

(event `Move Note`
  (bind _splinecomp (`self.SplineComp`))
  (`TimelineComponent.SetPlayRate` (`self.Timeline`) (/ 1.0 (`self.Time to Complete`)))
  (bind (_direction _newtrack_0) (`Timeline|Timeline` :!via `PlayFromStart`)
    (:`Update`
      (bind _returnvalue (`KismetMathLibrary.Lerp` 0.0 (`SplineComponent.GetSplineLength` (`self.SplineComp`)) _newtrack_0))
      (`self.K2_SetActorTransform` (`KismetMathLibrary.MakeTransform` (`SplineComponent.GetLocationAtDistanceAlongSpline` _splinecomp _returnvalue "World") (`SplineComponent.GetRotationAtDistanceAlongSpline` _splinecomp _returnvalue "World")))
      (`/Engine/EditorBlueprintResources/StandardMacros.DoOnce` false
        (:`Completed`
          (bind _returnvalue_2 (`AIBlueprintHelperLibrary.SpawnAIFromClass` "/Game/RhythmGame/Blueprints/BP_Enemy.BP_Enemy_C" null (`self.K2_GetActorLocation`) (`self.K2_GetActorRotation`) false null))
          (bind _asbp_enemy (cast `/Game/RhythmGame/Blueprints/BP_Enemy` _returnvalue_2))
          (set `/Game/RhythmGame/Blueprints/BP_Enemy.Spline Distance` (`SplineComponent.GetSplineLength` (`self.SplineComp`)) _asbp_enemy)
          (`/Game/RhythmGame/Blueprints/BP_Enemy.Move` _asbp_enemy))))
    (:`Finished`
      (`self.K2_DestroyActor`))))

(event `self.Sphere.OnComponentBeginOverlap`
  (params (OverlappedComponent :type "PrimitiveComponent Object Reference") (OtherActor :type "Actor Object Reference") (OtherComp :type "PrimitiveComponent Object Reference") (OtherBodyIndex :type Integer) (bFromSweep :type Boolean) (SweepResult :type "HitResult Structure (by ref)"))
  (cast `/Game/RhythmGame/Blueprints/BP_ThirdPersonCharacter` OtherActor)
  (`self.K2_DestroyActor`))

(fn `UserConstructionScript`)